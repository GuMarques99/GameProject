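; Final boss Blueprint that alternates charges at the player with bullet fire, triggered by a two-second loop from BeginPlay.
; Movement slides the capsule to the player character's location, then to an indexed MovingPoints entry, chaining three passes via a DoN counter before resetting.
; Bullet attack spawns BossBullet from BulletArrow at short intervals, capped at five by a DoN that is never reset here.
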(event Custom|Movemet
  (bind _capsulecomponent (Variables|Collision|GetCapsuleComponent))
  ;[1 1 1] Moving Attack
  (bind _counter (Utilities|DoN 3 :!label _label)
    (:Exit
      (bind _asbp_character (Utilities|Casting|CastToBP_CharacterClass "/Game/Blueprint/BP_Character.BP_Character_C"))
      (bind _returnvalue (Actor|GetActorOfClass _asbp_character))
      (bind _asbp_character_2 (Utilities|Casting|CastToBP_Character _returnvalue))
      (Components|MoveComponentTo _capsulecomponent (Transformation|GetActorLocation _asbp_character_2) "0, 0, 0" false false 1.0 false)
      (Components|MoveComponentTo _capsulecomponent (Utilities|Array|Get(acopy) (Variables|Default|GetMovingPoints) (- _counter 1)) "0, 0, 0" false false 2.0 false)
      (if (== _counter 3)
        (Utilities|FlowControl|Sequence
          (:then_0
            (goto _label Reset)))
        (else
          (goto _label))))))

(event Custom|Bullet_Attack
  (bind _bulletarrow (Variables|Default|GetBulletArrow))
  ;[1 1 1] Bullet Attack
  (Utilities|FlowControl|DoN 5 :!label _label
    (:Exit
      (Game|SpawnActorfromClass "/Game/Blueprint/BossBullet.BossBullet_C" (Math|Transform|MakeTransform (Transformation|GetWorldLocation _bulletarrow) (Transformation|GetWorldRotation _bulletarrow) "1,1,1") "Undefined" 0 0)
      (Utilities|FlowControl|Delay 0.2)
      (goto _label))))

(event EventBeginPlay
  (Utilities|FlowControl|Delay 2.0 :!label _label)
  (CallFunction|Movemet)
  (CallFunction|BulletAttack)
  (goto _label))

(event Collision|EventActorBeginOverlap
  (params (OtherActor :type Actor%20Object%20Reference)))

(event EventTick
  (params (DeltaSeconds :type Float%20%28single-precision%29)))

(fn ConstructionScript)