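; Fire trap actor that damages any BP_Character overlapping its Box by DamValueTrapOb and destroys itself 15 seconds after BeginPlay.
; Tick drives two chained 3-second Delays, one disabling the Box collision and clearing the Fire flipbook, the next restoring both.
; The Delays are re-triggered from Tick rather than run by a timer or loop, so the two phases are not strictly sequenced.
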(event OnComponentBeginOverlap(Box)
  (params (OverlappedComponent :type Primitive%20Component%20Object%20Reference) (OtherActor :type Actor%20Object%20Reference) (OtherComp :type Primitive%20Component%20Object%20Reference) (OtherBodyIndex :type Integer) (bFromSweep :type Boolean) (SweepResult :type Hit%20Result%20Structure%20%28by%20ref%29))
  (bind _asbp_character (Utilities|Casting|CastToBP_Character OtherActor))
  (Default|Damage _asbp_character (Variables|Default|GetDamValueTrapOb)))

(event EventBeginPlay
  (Utilities|FlowControl|Delay 15.0)
  (Actor|DestroyActor))

(event Collision|EventActorBeginOverlap
  (params (OtherActor :type Actor%20Object%20Reference)))

(event EventTick
  (params (DeltaSeconds :type Float%20%28single-precision%29))
  (Utilities|FlowControl|Delay 3.0)
  (Collision|SetCollisionEnabled (Variables|Default|GetBox) "NoCollision")
  (Sprite|SetFlipbook (Variables|Default|Getfire))
  (Utilities|FlowControl|Delay 3.0)
  (Collision|SetCollisionEnabled (Variables|Default|GetBox) "QueryOnly")
  (Sprite|SetFlipbook (Variables|Default|Getfire) "/Game/Sprites/Fire_Trap/Fire.Fire"))

(fn ConstructionScript)