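; Goblin enemy that moves back and forth and trades damage with BP_Character on contact.
; An interp movement component's reverse event toggles the Enemy component's yaw between 0 and 180 to turn it around.
; Box overlap hurts the goblin if the character is attacking, otherwise hurts the character.
; Taking damage applies a fixed impulse, prints remaining energy and destroys the actor at zero or below.
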(event OnInterptoReverse(EnemyMovement)
  (params (ImpactResult :type Hit%20Result%20Structure%20%28by%20ref%29) (Time :type Float%20%28single-precision%29))
  ;[1 1 1] Movement reverse
  (Math|Float|CompareFloat (Variables|Default|GetZ%20%28Yaw%29) 1.8e+02
    (:==
      (Variables|Default|SetZ%20%28Yaw%29 0.0))
    (:<
      (Variables|Default|SetZ%20%28Yaw%29 1.8e+02)))
  (Transformation|SetWorldRotation (Variables|Default|Getenemy) (Math|Rotator|MakeRotator 0.0 0.0 (Variables|Default|GetZ%20%28Yaw%29)) false false))

(event OnComponentBeginOverlap(Box)
  (params (OverlappedComponent :type Primitive%20Component%20Object%20Reference) (OtherActor :type Actor%20Object%20Reference) (OtherComp :type Primitive%20Component%20Object%20Reference) (OtherBodyIndex :type Integer) (bFromSweep :type Boolean) (SweepResult :type Hit%20Result%20Structure%20%28by%20ref%29))
  ;[1 1 1] Player collision
  (bind _asbp_character (Utilities|Casting|CastToBP_Character OtherActor))
  (if (Variables|/Game/Blueprint/BP_Character.BP_Character_C|Getattack _asbp_character)
    (CallFunction|Damage (Variables|/Game/Blueprint/BP_Character.BP_Character_C|GetForce _asbp_character))
    (else
      (Default|Damage _asbp_character (Variables|Default|GetGoblin%20Damage)))))

(event Custom|Damage
  (params (Damage%20suffered :type Float%20%28single-precision%29))
  ;[1 1 1] Damage and destroy
  (Physics|AddImpulse (Variables|Default|Getenemy) "10000.000000,0.0,10000.000000" "None" false)
  (bind _output_get (Variables|Default|SetGoblin%20Energy (- (Variables|Default|GetGoblin%20Energy) Damage%20suffered)))
  (Development|PrintString (Utilities|String|ToString(Float) (Variables|Default|GetGoblin%20Energy)))
  (Math|Float|CompareFloat _output_get 0.0
    (:==
      _)
    (:<
      _))
  (Actor|DestroyActor))

(event EventBeginPlay)

(event Collision|EventActorBeginOverlap
  (params (OtherActor :type Actor%20Object%20Reference)))

(event EventTick
  (params (DeltaSeconds :type Float%20%28single-precision%29)))

(fn ConstructionScript)